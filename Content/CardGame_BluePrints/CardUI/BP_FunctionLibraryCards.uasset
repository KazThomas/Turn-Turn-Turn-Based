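; Blueprint function library for the card game, providing random card draws and a movement helper for card widgets.
; Three pull functions each pick a random row from the Monster, Spell or Other card data table and return its data.
; InterpolateTowardsPos eases a widget transform's translation and angle toward a destination using delta time and a given speed, without carrying over scale or shear.
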(fn `InterpolateTowardsPos`
  (params (`Current Pos` :type "WidgetTransform Structure") (DestinationTransform :type "WidgetTransform Structure") (DeltaTime :type "Float (double-precision)") (InterpolationSpeed :type "Float (double-precision)"))
  (returns (`New Position` :type "WidgetTransform Structure"))
  (bind (_translation _scale _shear _angle) (break `WidgetTransform` `Current Pos`))
  (bind (_translation_2 _scale_2 _shear_2 _angle_2) (break `WidgetTransform` DestinationTransform))
  (bind _deltatime (`local.DeltaTime`))
  (bind _interpolationspeed (`local.InterpolationSpeed`))
  (return (make `WidgetTransform` (`KismetMathLibrary.Vector2DInterpTo` _translation _translation_2 _deltatime _interpolationspeed) (1.0 1.0) (0.0 0.0) (`KismetMathLibrary.FInterpTo` _angle _angle_2 _deltatime _interpolationspeed))))

(fn `Pull from Monster Table`
  (returns (CardInfo :type "/Game/CardGame_BluePrints/CardUI/DataTs+Structs/MonsterStructure Structure"))
  (bind _outrownames (`DataTableFunctionLibrary.GetDataTableRowNames` "/Game/CardGame_BluePrints/CardUI/DataTs+Structs/MonsterDataTable.MonsterDataTable"))
  (bind _returnvalue (`|GetDataTableRow` "/Game/CardGame_BluePrints/CardUI/DataTs+Structs/MonsterDataTable.MonsterDataTable" (`KismetArrayLibrary.Array_Random` _outrownames))
    (:`then`
      (return _returnvalue))
    (:`RowNotFound`
      (return))))

(fn `Pull from Other Table`
  (returns (CardInfo :type "/Game/CardGame_BluePrints/CardUI/DataTs+Structs/OtherCardStruct Structure"))
  (bind _outrownames (`DataTableFunctionLibrary.GetDataTableRowNames` "/Game/CardGame_BluePrints/CardUI/DataTs+Structs/OtherCardDataTable.OtherCardDataTable"))
  (bind _returnvalue (`|GetDataTableRow` "/Game/CardGame_BluePrints/CardUI/DataTs+Structs/OtherCardDataTable.OtherCardDataTable" (`KismetArrayLibrary.Array_Random` _outrownames))
    (:`then`
      (return _returnvalue))
    (:`RowNotFound`
      (return))))

(fn `Pull from Spell Table`
  (returns (CardInfo :type "/Game/CardGame_BluePrints/CardUI/DataTs+Structs/SpellStructure Structure"))
  (bind _outrownames (`DataTableFunctionLibrary.GetDataTableRowNames` "/Game/CardGame_BluePrints/CardUI/DataTs+Structs/SpellDataTable.SpellDataTable"))
  (bind _returnvalue (`|GetDataTableRow` "/Game/CardGame_BluePrints/CardUI/DataTs+Structs/SpellDataTable.SpellDataTable" (`KismetArrayLibrary.Array_Random` _outrownames))
    (:`then`
      (return _returnvalue))
    (:`RowNotFound`
      (return))))